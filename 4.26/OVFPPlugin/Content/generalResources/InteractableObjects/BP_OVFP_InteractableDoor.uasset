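; BP_OVFP_InteractableDoor is an interactable door that snaps between closed and open when it receives OVFPInteract.
; Interaction flips the Open flag and sets the Pivot's relative rotation to either zero or OpenRotationOffset, with no animation.
; The construction script applies the same rotation from Open, and the interact path transacts the actor and refreshes the editor viewport, suggesting it also supports toggling in the editor.
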(event `/OVFPPlugin/generalResources/InteractableObjects/Utilities/BPI_OVFP_InteractInterface.OVFP_Interact`
  (bind _pivot (`self.Pivot`))
  (if (`self.Open?`) :!label _label
    (`SceneComponent.K2_SetRelativeRotation` :`self` _pivot)
    (set `self.Open?` false)
    (else
      (`SceneComponent.K2_SetRelativeRotation` _pivot (`self.Open Rotation Offset`) false false)
      (set `self.Open?` true)))
  (`KismetSystemLibrary.TransactObject` self)
  (`VPBlueprintLibrary.Refresh3DEditorViewport`))

(event `OVFPInteract`
  (goto _label))

(fn `UserConstructionScript`
  (bind _pivot (`self.Pivot`))
  (if (`self.Open?`)
    (`SceneComponent.K2_SetRelativeRotation` _pivot (`self.Open Rotation Offset`) false false)
    (else
      (`SceneComponent.K2_SetRelativeRotation` :`self` _pivot))))