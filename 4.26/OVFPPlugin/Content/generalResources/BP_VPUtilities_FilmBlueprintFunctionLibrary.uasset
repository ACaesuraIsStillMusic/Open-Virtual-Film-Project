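; Blueprint function library of general-purpose helpers for film and virtual production (VP) work.
; Math functions remap ranges, convert lens millimetres to and from horizontal FOV using filmback and anamorphic squeeze, and convert length and speed units.
; Array and string helpers insert actors, insertion-sort them by display name, increment numeric suffixes and split quoted CSV lines.
; An editor-side helper imports and saves an image through an automated AssetTools task, returning the new asset path.
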(fn `ParseCSVStringIntoArray`
  (params (`Source String` :type String))
  (returns (Array :type "Array of String"))
  (locals (TempArray :type "Array of String") (TempString :type String) (`Out Array` :type "Array of String") (Quoting :type Boolean))
  (if (`KismetStringLibrary.Contains` `Source String` "\",")
    (set `local.TempArray` (`KismetStringLibrary.ParseIntoArray` `Source String` "\"," false))
    (for _array_element (`local.TempArray`)
      (bind (_lefts _rights _returnvalue) (`KismetStringLibrary.Split` _array_element ",\""))
      (if _returnvalue
        (`KismetArrayLibrary.Array_Append` (`local.Out Array`) (`KismetStringLibrary.ParseIntoArray` _lefts "," false))
        (`KismetArrayLibrary.Array_Add` (`local.Out Array`) _rights)
        (else
          ;[1 1 1] Only 1 term, remove any extra "
          (`KismetArrayLibrary.Array_Add` (`local.Out Array`) (`KismetStringLibrary.Replace` _array_element "\"")))))
    (else
      (set `local.Out Array` (`KismetStringLibrary.ParseIntoArray` `Source String` "," false))))
  (return (`local.Out Array`)))

(fn `VP_AddActorToArrayAtLocation`
  (params (`Input Array` :type "Array of Actor Object Reference") (`Index To Add` :type Integer) (`Acror To Add` :type "Actor Object Reference"))
  (returns (OutputArray1 :type "Array of Actor Object Reference"))
  (locals (OutputArray :type "Array of Actor Object Reference"))
  (bind _outputarray (`local.OutputArray`))
  (if (>= `Index To Add` (- (`KismetArrayLibrary.Array_Length` `Input Array`) 1))
    (bind _output_get (set `local.OutputArray` `Input Array`))
    (`KismetArrayLibrary.Array_Add` _output_get `Acror To Add`)
    (else
      (`KismetArrayLibrary.Array_Clear` (`local.OutputArray`))
      (for (_array_element _array_index) `Input Array`
        (if (== _array_index `Index To Add`)
          (`KismetArrayLibrary.Array_Add` _outputarray `Acror To Add`))
        (`KismetArrayLibrary.Array_Add` _outputarray _array_element))))
  (return (`local.OutputArray`)))

(fn `VP_ConvertLength`
  (params (`Input Value` :type "Float (double-precision)") (`Input Unit` :type "/OVFPPlugin/generalResources/Enum/VPUtilities_UnitsLength-OVFP Enum" :default "NewEnumerator0"))
  (returns (Miles1 :type "Float (double-precision)") (`Feet and Inches` :type Text) (Feet1 :type "Float (double-precision)") (Inches1 :type "Float (double-precision)") (Kilometers1 :type "Float (double-precision)") (Meters1 :type "Float (double-precision)") (Centimeters1 :type "Float (double-precision)"))
  (locals (Measure_Unit_Conversion :type "Float (double-precision)") (Miles :type "Float (double-precision)") (Feet :type "Float (double-precision)") (Inches :type "Float (double-precision)") (Meters :type "Float (double-precision)") (Kilometers :type "Float (double-precision)") (Centimeters :type "Float (double-precision)") (InputValueForConversion :type "Float (double-precision)"))
  (bind _feet (`local.Feet`))
  (set `local.InputValueForConversion` `Input Value`)
  (switch `/OVFPPlugin/generalResources/Enum/VPUtilities_UnitsLength-OVFP` `Input Unit`
    (:`NewEnumerator0`
      (set `local.Measure_Unit_Conversion` 30.48))
    (:`NewEnumerator3`
      (set `local.Measure_Unit_Conversion` 2.54))
    (:`NewEnumerator4`
      (set `local.Measure_Unit_Conversion` 100.0))
    (:`NewEnumerator5`
      (set `local.Measure_Unit_Conversion` 1.0))
    (:`NewEnumerator6`
      (set `local.Measure_Unit_Conversion` 160934.40625))
    (:`NewEnumerator7`
      (set `local.Measure_Unit_Conversion` 100000.0)))
  (set `local.Miles` (/ (* (`local.InputValueForConversion`) (`local.Measure_Unit_Conversion`)) 160934.40625))
  (set `local.Feet` (/ (* (`local.InputValueForConversion`) (`local.Measure_Unit_Conversion`)) 30.48))
  (set `local.Inches` (* (`local.Feet`) 12.0))
  (set `local.Meters` (/ (* (`local.InputValueForConversion`) (`local.Measure_Unit_Conversion`)) 100.0))
  (set `local.Kilometers` (/ (* (`local.InputValueForConversion`) (`local.Measure_Unit_Conversion`)) 100000.0))
  (set `local.Centimeters` (* (`local.InputValueForConversion`) (`local.Measure_Unit_Conversion`)))
  (return (`local.Miles`) (`|FormatText` "{feet}' {inches}\"" (`KismetMathLibrary.FFloor` _feet) (* (`KismetMathLibrary.Fraction` _feet) 12.0)) _feet (`local.Inches`) (`local.Kilometers`) (`local.Meters`) (`local.Centimeters`)))

(fn `VP_ConvertSpeed`
  (params (`Input Speed` :type "Float (double-precision)") (`Input Units` :type "/OVFPPlugin/generalResources/Enum/VPUtilities_UnitsSpeed-OVFP Enum" :default "NewEnumerator0"))
  (returns (`cm/s` :type "Float (double-precision)") (`M/s` :type "Float (double-precision)") (`Km/h` :type "Float (double-precision)") (`ft/s` :type "Float (double-precision)") (Mph :type "Float (double-precision)"))
  (bind _returnvalue (/ `Input Speed` (select `/OVFPPlugin/generalResources/Enum/VPUtilities_UnitsSpeed-OVFP` `Input Units` :`NewEnumerator0` 1.0 :`NewEnumerator1` 0.01 :`NewEnumerator2` 0.036 :`NewEnumerator3` 0.032808 :`NewEnumerator4` 0.022369 :!type "Float (single-precision)")))
  (return _returnvalue (* _returnvalue 0.01) (* _returnvalue 0.036) (* _returnvalue 0.032808) (* _returnvalue 0.022369)))

(fn `VP_HorizontalFOV to LensMM`
  (params (`Filmback W` :type "Float (double-precision)") (AnamorphicSqueeze :type "Float (double-precision)" :default 1.0) (FOV :type "Float (double-precision)"))
  (returns (LensMM :type "Float (double-precision)"))
  (return (/ (* `Filmback W` AnamorphicSqueeze) (* 2.0 (`KismetMathLibrary.DegTan` (/ FOV 2.0))))))

(fn `VP_ImportImage`
  (params (SelfReference :type "Object Object Reference") (Filename :type String) (DestinationPath :type String))
  (returns (ImagePath :type String))
  (locals (TaskArray :type "Array of AssetImportTask Object Reference"))
  (bind _taskarray (`local.TaskArray`))
  (bind _importedobjectpaths (`AssetImportTask.ImportedObjectPaths` (`|GetArrayItem` _taskarray)))
  (bind _returnvalue (`AssetToolsHelpers.GetAssetTools`))
  (`KismetArrayLibrary.Array_Clear` (`local.TaskArray`))
  (bind _returnvalue_2 (`|GenericCreateObject` "/Script/UnrealEd.AssetImportTask" SelfReference))
  (`|ExecutionSequence`
    (:`then_0`
      (bind _output_get (set `AssetImportTask.Filename` Filename _returnvalue_2)))
    (:`then_1`
      (set `AssetImportTask.DestinationPath` DestinationPath _returnvalue_2))
    (:`then_2`
      (set `AssetImportTask.bReplaceExisting` false _returnvalue_2))
    (:`then_3`
      (set `AssetImportTask.bAutomated` true _returnvalue_2))
    (:`then_4`
      (set `AssetImportTask.bSave` true _returnvalue_2))
    (:`then_5`
      ;[1 1 1] Add 1 task for each texture
      (`KismetArrayLibrary.Array_Add` _taskarray _returnvalue_2)
      (if (> (`KismetStringLibrary.Len` _output_get) 0)
        (`AssetTools.ImportAssetTasks` _returnvalue _taskarray)
        (if (> (`KismetArrayLibrary.Array_Length` _importedobjectpaths) 0)
          (return (`|GetArrayItem` _importedobjectpaths)))))))

(fn `VP_IncrementStringSuffix`
  (params (SourceString :type String))
  (returns (`Output String` :type String))
  (bind _returnvalue (`KismetStringLibrary.Conv_StringToInt` (`KismetStringLibrary.Reverse` SourceString)))
  (bind _returnvalue_2 (`KismetStringLibrary.Reverse` (`KismetStringLibrary.Conv_IntToString` _returnvalue)))
  (return (`KismetStringLibrary.Concat_StrStr` (`KismetStringLibrary.GetSubstring` SourceString 0 (- (`KismetStringLibrary.Len` SourceString) (select `bool` (== _returnvalue 0) :`false` (`KismetStringLibrary.Len` _returnvalue_2)))) (`KismetStringLibrary.Conv_IntToString` (+ (`KismetStringLibrary.Conv_StringToInt` _returnvalue_2) 1)))))

(fn `VP_Lens MM to Horizontal FOV`
  (params (`Lens MM` :type "Float (double-precision)") (`Filmback W` :type "Float (double-precision)") (AnamorphicSqueeze :type "Float (double-precision)" :default 1.0))
  (returns (FOV :type "Float (double-precision)"))
  (return (* 2.0 (`KismetMathLibrary.DegAtan` (/ (* `Filmback W` AnamorphicSqueeze) (* 2.0 `Lens MM`))))))

(fn `VP_Remap Float To Range`
  (params (Value :type "Float (double-precision)") (`In Min` :type "Float (double-precision)") (`In Max` :type "Float (double-precision)") (`Out Min ` :type "Float (double-precision)") (`Out Max` :type "Float (double-precision)"))
  (returns (Output :type "Float (double-precision)"))
  (return (+ (* (/ (- Value `In Min`) (- `In Max` `In Min`)) (- `Out Max` `Out Min `)) `Out Min `)))

(fn `VP_SortActorsInArrayByName`
  (params (Actors :type "Array of Actor Object Reference"))
  (returns (`Sorted Actors` :type "Array of Actor Object Reference"))
  (locals (ArraySorted :type "Array of Actor Object Reference") (SortIndex :type Integer) (LetterIndexTemp :type Integer))
  (bind _sortindex (`local.SortIndex`))
  (bind _letterindextemp (`local.LetterIndexTemp`))
  (bind _arraysorted (`local.ArraySorted`))
  (bind _letterindextemp_2 (`local.LetterIndexTemp`))
  (for _array_element Actors
    (for (_array_element_2 _array_index) (`local.ArraySorted`)
      (set `local.SortIndex` _array_index)
      (set `local.LetterIndexTemp` 0)
      (bind _returnvalue (`KismetStringLibrary.ToUpper` (`KismetSystemLibrary.GetDisplayName` _array_element_2)))
      (bind _returnvalue_2 (`KismetStringLibrary.GetCharacterAsNumber` _returnvalue _letterindextemp))
      (bind _returnvalue_3 (`KismetStringLibrary.ToUpper` (`KismetSystemLibrary.GetDisplayName` _array_element)))
      (while (and (== _returnvalue_2 (`KismetStringLibrary.GetCharacterAsNumber` _returnvalue_3 _letterindextemp)) (!= _returnvalue_2 0))
        (`/Engine/EditorBlueprintResources/StandardMacros.IncrementInt` (`local.LetterIndexTemp`)))
      (if (< (`KismetStringLibrary.GetCharacterAsNumber` _returnvalue_3 _letterindextemp_2) (`KismetStringLibrary.GetCharacterAsNumber` _returnvalue _letterindextemp_2))
        (break)
        (else
          (`/Engine/EditorBlueprintResources/StandardMacros.IncrementInt` (`local.SortIndex`)))))
    (if (>= _sortindex (`KismetArrayLibrary.Array_Length` (`local.ArraySorted`)))
      (`KismetArrayLibrary.Array_Add` _arraysorted _array_element)
      (else
        (`KismetArrayLibrary.Array_Insert` _arraysorted _array_element _sortindex))))
  (return (`local.ArraySorted`)))